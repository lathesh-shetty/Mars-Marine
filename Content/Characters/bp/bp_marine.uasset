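; Player marine character for a twin-stick style shooter, with world-axis movement, a HUD widget, clamped health, death state and kill counter.
; Aim sets control yaw from either gamepad thumbstick or smoothed mouse velocity, both deadzoned, switching on the last key's device.
; Firing toggles muzzle effect and sound, while a looping timer runs hitscan traces from the muzzle socket along control rotation, applying damage and impact particles.
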(event `self.ReceiveBeginPlay`
  (bind _returnvalue (`|CreateWidget` "/Game/UI/W_playerHUD.W_playerHUD_C" null self))
  (`UserWidget.AddToViewport` _returnvalue 0))

(event `InputAxis|MoveForward`
  (params (AxisValue :type "Float (single-precision)"))
  (if (`self.is alive`)
    (`self.AddMovementInput` (1.0 0.0 0.0) AxisValue)))

(event `InputAxis|MoveRight`
  (params (AxisValue :type "Float (single-precision)"))
  (if (`self.is alive`)
    (`self.AddMovementInput` (0.0 1.0 0.0) AxisValue)))

(event `self.ReceiveTick`
  (params (DeltaSeconds :type "Float (single-precision)"))
  (`|ExecutionSequence`
    (:`then_0`
      (`self.update player aim`))))

(event `Key|AnyKey`
  (params (Key :type "Key Structure"))
  (:`Pressed`
    (set `self.mouse_or_thumbstick` (`KismetInputLibrary.Key_IsGamepadKey` Key))))

(event `InputAction|fire weapon`
  (params (Key :type "Key Structure"))
  (:`Pressed`
    (`self.start firing`)
    (`self.weapon trace`))
  (:`Released`
    (`self.stop firing`)))

(event `self.ReceiveAnyDamage`
  (params (Damage :type "Float (single-precision)") (DamageType :type "DamageType Object Reference") (InstigatedBy :type "Controller Object Reference") (DamageCauser :type "Actor Object Reference"))
  (if (`self.is alive`)
    (bind _health (`self.Decrease health` Damage))
    (if (== _health 0.0)
      (set `self.Dead` true)
      (`self.stop firing`))))

(fn `add health`
  (params (`health to add` :type "Float (double-precision)"))
  (set `self.health` (`KismetMathLibrary.FClamp` (+ (`self.health`) `health to add`) 0.0 100.0)))

(fn `Decrease health`
  (params (`Damage amount` :type "Float (double-precision)"))
  (returns (Health :type "Float (double-precision)"))
  (bind _output_get (set `self.health` (`KismetMathLibrary.FClamp` (- (`self.health`) `Damage amount`) 0.0 100.0)))
  (return _output_get))

(fn `GET MOUSE AIM DIRECTION`
  (returns (ReturnValue :type "Rotator Structure"))
  (bind (_returnvalue_x _returnvalue_y) (`KismetMathLibrary.BreakVector2D` (`self.get mouse velocity`)))
  (return (`KismetMathLibrary.RInterpTo` (`Controller.GetControlRotation` (`GameplayStatics.GetPlayerController` 0)) (`KismetMathLibrary.MakeRotator` 0.0 0.0 (`KismetMathLibrary.DegAtan2` _returnvalue_x _returnvalue_y)) (`GameplayStatics.GetWorldDeltaSeconds`) (`self.mouse smoothing strength`))))

(fn `get mouse velocity`
  (returns (ReturnValue :type "Vector2D Structure"))
  (bind (_deltax _deltay) (`PlayerController.GetInputMouseDelta` (`GameplayStatics.GetPlayerController` 0)))
  (return (/ (`KismetMathLibrary.MakeVector2D` _deltax _deltay) (`GameplayStatics.GetWorldDeltaSeconds`))))

(fn `get weapon trace end location`
  (returns (ReturnValue :type "Vector Structure"))
  (return (+ (`self.get weapon trace start location`) (* (`KismetMathLibrary.GetForwardVector` (`self.GetControlRotation`)) (`self.weapon range`)))))

(fn `get weapon trace start location`
  (returns (ReturnValue :type "Vector Structure"))
  (return (`SceneComponent.GetSocketLocation` (`self.P_AssaultRifle_MF`) "MuzzleFlashSocket")))

(fn `increase kill`
  (`/Engine/EditorBlueprintResources/StandardMacros.IncrementFloat` (`self.kill`)))

(fn `is aim above deadzone`
  (returns (ReturnValue :type Boolean))
  (return (> (`KismetMathLibrary.VSize2D` (`KismetMathLibrary.MakeVector2D` (`self.GetInputAxisValue`) (`self.GetInputAxisValue`))) (`self.thumbstick_Aim_deadzone`))))

(fn `is alive`
  (returns (`not dead` :type Boolean))
  (return (not (`self.Dead`))))

(fn `is health full`
  (returns (ReturnValue :type Boolean))
  (return (== (`self.health`) 100.0)))

(fn `is mouse deadzone`
  (returns (ReturnValue :type Boolean))
  (return (> (`KismetMathLibrary.VSize2D` (`self.get mouse velocity`)) (`self.mouse_deadzone`))))

(fn `spawn impact hit`
  (params (`hit Location` :type "Vector Structure"))
  (`GameplayStatics.SpawnEmitterAtLocation` "/Game/Effects/Weapons/Impacts/P_AssaultRifle_IH.P_AssaultRifle_IH" `hit Location`))

(fn `start firing`
  (if (`self.is alive`)
    (`ActorComponent.Activate` (`self.P_AssaultRifle_MF`) false)
    (bind _returnvalue (`GameplayStatics.SpawnSound2D` "/Game/Sounds/Weapon_AssaultRifle/Stereo/rifle_cue.rifle_cue" 1.0 1.0 0.0 null))
    (set `self.Weapon fire sound` _returnvalue)
    (`self.weapon trace`)
    (`KismetSystemLibrary.K2_SetTimer` null "weapon trace" (`self.weapon fire rate`) true)))

(fn `stop firing`
  (bind _weapon_fire_sound (`self.Weapon fire sound`))
  (`ActorComponent.Deactivate` (`self.P_AssaultRifle_MF`))
  (`/Engine/EditorBlueprintResources/StandardMacros.IsValid` _weapon_fire_sound
    (:`Is Valid`
      (`AudioComponent.Stop` _weapon_fire_sound)
      (`KismetSystemLibrary.K2_ClearTimer` null "weapon trace")
      (if (`self.is alive`)
        (`GameplayStatics.SpawnSound2D` "/Game/Sounds/Weapon_AssaultRifle/Stereo/riflefireend_cue.riflefireend_cue" 1.0 1.0 0.0 null)))))

(fn `thumbstick aim direction]`
  (returns (ReturnValue :type "Rotator Structure"))
  (return (`KismetMathLibrary.MakeRotator` 0.0 0.0 (`KismetMathLibrary.DegAtan2` (`self.GetInputAxisValue`) (`self.GetInputAxisValue`)))))

(fn `update mouse aim`
  (if (`self.is mouse deadzone`)
    (`Controller.SetControlRotation` (`GameplayStatics.GetPlayerController` 0) (`self.GET MOUSE AIM DIRECTION`))))

(fn `update player aim`
  (if (`self.is alive`)
    (if (`self.mouse_or_thumbstick`)
      (`self.update thumbstick aim`)
      (else
        (`self.update mouse aim`)))))

(fn `update thumbstick aim`
  (if (`self.is aim above deadzone`)
    (`Controller.SetControlRotation` (`GameplayStatics.GetPlayerController` 0) (`self.thumbstick aim direction]`))))

(fn `UserConstructionScript`)

(fn `weapon trace`
  (bind _outhit (`KismetSystemLibrary.LineTraceSingle` (`self.get weapon trace start location`) (`self.get weapon trace end location`) "TraceTypeQuery1"))
  (bind (_bblockinghit _binitialoverlap _time _distance _location _impactpoint _normal _impactnormal _physmat _hitactor) (`GameplayStatics.BreakHitResult` _outhit))
  (if _bblockinghit
    (`self.spawn impact hit` _location)
    (`GameplayStatics.ApplyDamage` _hitactor (`self.damage per shot`))))