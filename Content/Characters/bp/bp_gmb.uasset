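; Wave manager Blueprint (likely the game mode) that runs endless, escalating alien waves, starting shortly after BeginPlay.
; Each wave multiplies the difficulty to set the spawn count, then a looping timer spawns aliens at random TargetPoints until the count runs out.
; Spawned aliens are tracked in an array; RegisterAlienDeath removes them and, once none remain alive or pending, ends the wave, starting the next after a delay.
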(event `self.ReceiveBeginPlay`
  (`KismetSystemLibrary.Delay` 2.0)
  (`self.start new wave`))

(event `spawn wave`
  (`self.spawn alien`))

(event `end wave`
  (`KismetSystemLibrary.Delay` 2.0)
  (`self.start new wave`))

(event `self.ReceiveTick`
  (params (DeltaSeconds :type "Float (single-precision)")))

(fn `get random spawn point`
  (returns (`Spawn point` :type "TargetPoint Object Reference"))
  (bind _outactors (`GameplayStatics.GetAllActorsOfClass` "/Script/Engine.TargetPoint"))
  (return (`|GetArrayItem` _outactors (`KismetMathLibrary.RandomIntegerInRange` 0 (`KismetArrayLibrary.Array_LastIndex` _outactors)))))

(fn `INCREASE WAVE difficulty`
  (bind _output_get (set `self.wave dificulty` (`KismetMathLibrary.Round` (* (`self.wave dificulty`) (`self.difficulty multiplier`)))))
  (set `self.Alien spawn remaining` _output_get))

(fn `is wave complete`
  (returns (ReturnValue :type Boolean))
  (return (and (== (`KismetArrayLibrary.Array_Length` (`self.Aliens`)) 0) (== (`self.Alien spawn remaining`) 0))))

(fn `register alien death`
  (params (Alien :type "/Game/Characters/bp/ai/bp_alien Object Reference (by ref)"))
  (`KismetArrayLibrary.Array_RemoveItem` (`self.Aliens`) Alien)
  (if (`self.is wave complete`)
    (`self.end wave`)))

(fn `spawn alien`
  (bind _spawn_point (`self.get random spawn point`))
  (`/Engine/EditorBlueprintResources/StandardMacros.IsValid` _spawn_point
    (:`Is Valid`
      (bind _returnvalue (`|SpawnActorFromClass` "/Game/Characters/bp/ai/bp_alien.bp_alien_C" (`self.GetTransform` _spawn_point) "Undefined" "OverrideRootScale" null null))
      (`/Engine/EditorBlueprintResources/StandardMacros.IsValid` _returnvalue
        (:`Is Valid`
          (`KismetArrayLibrary.Array_Add` (`self.Aliens`) _returnvalue)
          (bind _result (`/Engine/EditorBlueprintResources/StandardMacros.DecrementInt` (`self.Alien spawn remaining`))
            (:`  `
              (if (== _result 0)
                (`KismetSystemLibrary.K2_ClearTimer` null "spawn wave")))))))))

(fn `start new wave`
  (`/Engine/EditorBlueprintResources/StandardMacros.IncrementInt` (`self.current wave`)
    (:`  `
      (`self.INCREASE WAVE difficulty`)
      (`KismetSystemLibrary.K2_SetTimer` null "spawn wave" 1.0 true))))

(fn `UserConstructionScript`)